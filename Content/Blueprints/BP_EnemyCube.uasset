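; BP_EnemyCube is a damageable enemy cube with a floating health bar that can optionally move along a looping path.
; Damage lowers Health, updates the BP_EnemyHealthBar widget and destroys the actor once health drops below zero.
; When IsMoving is set, a Timeline scaled by MovementTime lerps it from its start location by the EndLocation offset, restarting each cycle.
; Every tick the health bar widget rotates to face the player character.
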(event Custom|StartMovement
  (bind _startlocation (Variables|Default|GetStartLocation))
  (bind _newtrack_1 (Timeline|Timeline Play)
    (:Update
      (Transformation|SetActorLocation (Math|Vector|Lerp(Vector) _startlocation (+ _startlocation (Variables|Default|GetEndLocation)) _newtrack_1) false true))
    (:Finished
      (Utilities|FlowControl|DelayUntilNextTick)
      (Timeline|Timeline PlayFromStart))))

(event Custom|TakeDamage
  (params (Damage :type Float%20%28double-precision%29))
  (bind _output_get (Variables|Default|SetHealth (- (Variables|Default|GetHealth) Damage)))
  (Variables|/Game/Blueprints/BP_EnemyHealthBar.BP_EnemyHealthBar_C|SetHealthValue (Variables|Default|GetAs%20BP%20Enemy%20Health%20Bar) _output_get)
  (if (< (Variables|Default|GetHealth) 0.0)
    (Actor|DestroyActor)))

(event EventBeginPlay
  (Variables|Default|SetStartLocation (Transformation|GetActorLocation))
  (Variables|Default|SetHealth (Variables|Default|GetMaxHealth))
  (bind _asbp_enemy_health_bar (Utilities|Casting|CastToBP_EnemyHealthBar (UserInterface|GetUserWidgetObject (Variables|Default|GetWidget))))
  (Variables|Default|SetAs%20BP%20Enemy%20Health%20Bar _asbp_enemy_health_bar)
  (Components|Timeline|SetPlayRate (Variables|Default|GetTimeline) (/ 1.0 (Variables|Default|GetMovementTime)))
  (if (Variables|Default|GetIsMoving)
    (CallFunction|StartMovement)))

(event EventTick
  (params (DeltaSeconds :type Float%20%28single-precision%29))
  (Transformation|SetWorldRotation (Variables|Default|GetWidget) (Math|Rotator|FindLookatRotation (Transformation|GetWorldLocation (Variables|Default|GetWidget)) (Transformation|GetActorLocation (Game|GetPlayerCharacter 0))) false false))

(fn ConstructionScript)
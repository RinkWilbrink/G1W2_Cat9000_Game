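; Dynamite projectile actor that explodes on a timed fuse or on impact.
; BeginPlay starts a five-second fuse shortened by InitialTimer, and hits trigger an earlier explosion unless IsBouncy is set or the first-person character is struck.
; Explode only prints a debug string and destroys the actor, with no damage or effects.
; The construction script feeds InitialSpeed into the projectile movement component.
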(event Custom|Explode
  (Development|PrintString "KABOOM")
  (Actor|DestroyActor))

(event EventBeginPlay
  (Utilities|FlowControl|Delay (- 5.0 (Variables|Default|GetInitialTimer)))
  (CallFunction|Explode))

(event Collision|EventHit
  (params (MyComp :type Primitive%20Component%20Object%20Reference) (Other :type Actor%20Object%20Reference) (OtherComp :type Primitive%20Component%20Object%20Reference) (bSelfMoved :type Boolean) (HitLocation :type Vector :default "0, 0, 0") (HitNormal :type Vector :default "0, 0, 0") (NormalImpulse :type Vector :default "0, 0, 0") (Hit :type Hit%20Result%20Structure%20%28by%20ref%29))
  (Utilities|Casting|CastToBP_FirstPersonCharacter Other
    (:CastFailed
      (if (not (Variables|Default|GetIsBouncy))
        (CallFunction|Explode)))))

(fn ConstructionScript
  (Variables|/Script/Engine.ProjectileMovementComponent|SetInitialSpeed (Variables|Default|GetProjectileMovement) (Variables|Default|GetInitial%20Speed)))
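; BP_Dynamite is a timed explosive that pushes first-person characters caught in its blast radius.
; OnInstantiate sets the fuse to the delay minus time already cooked and stores an explode-on-impact flag, unused here.
; Tick counts down and calls OnExplode, which repeats every frame after expiry as nothing stops it.
; OnExplode sphere-overlaps actors and adds force along each character's forward vector, not away from the blast.
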(event EventBeginPlay)

(event EventTick
  (params (DeltaSeconds :type Float%20%28single-precision%29))
  (if (>= (Variables|Default|Getm_CookDelayTime) (Variables|Default|Getm_CookTimer))
    (Variables|Default|Setm_CookTimer (- (Variables|Default|Getm_CookTimer) DeltaSeconds))
    (if (<= (Variables|Default|Getm_CookTimer) 0.0)
      (CallFunction|OnExplode))))

(fn ConstructionScript)

(fn OnInstantiate
  (params (_CookTime :type Float%20%28double-precision%29) (_ExplodeOnImpact :type Boolean))
  (Variables|Default|Setm_CookTimer (- (Variables|Default|Getm_CookDelayTime) _CookTime))
  (Variables|Default|Setm_ExplodeOnImpact _ExplodeOnImpact))

(fn OnExplode
  (bind _m_addforcestrength (Variables|Default|Getm_AddForceStrength))
  (bind _returnvalue (Math|Conversions|ToVector(Float) _m_addforcestrength))
  (Development|PrintText "Exploded!" true true "(R=1.000000,G=0.000000,B=0.000000,A=1.000000)")
  (bind (_outactors _returnvalue_2) (Collision|SphereOverlapActors (Transformation|GetActorLocation) (Variables|Default|Getm_ExplosionRadius) (Utilities|Array|MakeArray "ObjectTypeQuery2" "ObjectTypeQuery3") 0))
  (if _returnvalue_2
    (for _array_element _outactors
      (bind _asbp_first_person_character (Utilities|Casting|CastToBP_FirstPersonCharacter _array_element)
        (:then
          (Physics|AddForce (Variables|/Script/Engine.Character|GetCharacterMovement _asbp_first_person_character) (* (Transformation|GetActorForwardVector _asbp_first_person_character) _returnvalue))
          (Development|PrintString (Utilities|String|ToString(Vector) _returnvalue)))
        (:CastFailed
          (Development|PrintText "Failed to cast to character"))))))